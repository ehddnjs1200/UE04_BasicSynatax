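; Chest actor with a hinged skeletal-mesh head that opens and closes through its Open event.
; Open plays or reverses the OpenHead timeline based on IsOpen, pitching the head as it updates and flipping IsOpen when finished.
; The construction script applies a shared dynamic instance of MI_Chest to head and body, tinting its Emissive parameter with ChestColor.
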(event `self.ReceiveBeginPlay`)

(event `self.Open`
  (if (`self.bIsOpen`)
    (bind (_direction _speed) (`Timeline|OpenHead` :!via `Reverse` :!label _label)
      (:`Update`
        (`SceneComponent.K2_SetRelativeRotation` (`self.SkeletalMesh_Head`) (`KismetMathLibrary.MakeRotator` 0.0 (`KismetMathLibrary.Lerp` 0.0 140.0 _speed)) false false))
      (:`Finished`
        (if (`self.bIsOpen`)
          (set `self.bIsOpen` false)
          (else
            (set `self.bIsOpen` true)))))
    (else
      (goto _label))))

(fn `UserConstructionScript`
  (bind _returnvalue (`KismetMaterialLibrary.CreateDynamicMaterialInstance` "/Game/Assignment/Chest/MI_Chest.MI_Chest"))
  (`PrimitiveComponent.SetMaterial` (`self.SkeletalMesh_Head`) 0 _returnvalue)
  (`PrimitiveComponent.SetMaterial` (`self.SkeletalMesh_Body`) 0 _returnvalue)
  (`MaterialInstanceDynamic.SetVectorParameterValue` _returnvalue "Emissive" (`self.ChestColor`)))